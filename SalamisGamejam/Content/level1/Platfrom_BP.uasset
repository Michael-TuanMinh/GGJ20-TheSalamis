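; Platform actor that toggles whether its Box collides with pawns, based on the player's presence in a trigger volume.
; Box ignores the Pawn channel from BeginPlay, blocks it when the player character begins overlapping Box1, and ignores it again when that overlap ends.
; A height comparison between the player's mesh and Box runs on overlap, but both branches are empty, so it does not affect the result.
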(event OnComponentBeginOverlap(Box1)
  (params (OverlappedComponent :type Primitive%20Component%20Object%20Reference) (OtherActor :type Actor%20Object%20Reference) (OtherComp :type Primitive%20Component%20Object%20Reference) (OtherBodyIndex :type Integer) (bFromSweep :type Boolean) (SweepResult :type Hit%20Result%20Structure%20%28by%20ref%29))
  (bind _returnvalue (Game|GetPlayerCharacter 0))
  (bind _box (Variables|Default|GetBox))
  (if (== OtherActor _returnvalue)
    (if (> (.Z (Math|Vector|BreakVector (Transformation|GetWorldLocation (Variables|/Script/Engine.Character|GetMesh _returnvalue)))) (.Z (Math|Vector|BreakVector (Transformation|GetWorldLocation _box))))
      _
      (else
        _))
    (Collision|SetCollisionResponsetoChannel _box "ECC_Pawn" "ECR_Block")))

(event OnComponentEndOverlap(Box1)
  (params (OverlappedComponent :type Primitive%20Component%20Object%20Reference) (OtherActor :type Actor%20Object%20Reference) (OtherComp :type Primitive%20Component%20Object%20Reference) (OtherBodyIndex :type Integer))
  (if (== OtherActor (Game|GetPlayerCharacter 0))
    (Collision|SetCollisionResponsetoChannel (Variables|Default|GetBox) "ECC_Pawn" "ECR_Ignore")))

(event EventBeginPlay
  (Collision|SetCollisionResponsetoChannel (Variables|Default|GetBox) "ECC_Pawn" "ECR_Ignore"))

(event Collision|EventActorBeginOverlap
  (params (OtherActor :type Actor%20Object%20Reference)))

(event EventTick
  (params (DeltaSeconds :type Float%20%28single-precision%29)))

(fn ConstructionScript)